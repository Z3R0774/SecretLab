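; BP_Drifter is an actor whose Sphere component drifts back and forth along the X axis.
; Each Tick offsets the sphere's relative location at a constant, delta-time-scaled speed, with the boolean NewVar0 selecting the direction.
; The flag flips when the sphere's world X passes either of two hardcoded limits, so the travel range is fixed in world space rather than relative to the actor.
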(event EventTick
  (params (DeltaSeconds :type Float%20%28single-precision%29))
  (if (Variables|Default|GetNewVar_0)
    (Transformation|AddRelativeLocation (Variables|Default|GetSphere) (Math|Vector|MakeVector (* DeltaSeconds 5e+02) 0.0 0.0) false false)
    (if (not (<= (.x (Transformation|GetWorldLocation (Variables|Default|GetSphere))) 6.1e+03))
      (Variables|Default|SetNewVar_0 false))
    (else
      (Transformation|AddRelativeLocation (Variables|Default|GetSphere) (Math|Vector|MakeVector (* DeltaSeconds -5e+02) 0.0 0.0) false false)
      (if (not (>= (.x (Transformation|GetWorldLocation (Variables|Default|GetSphere))) 4e+03))
        (Variables|Default|SetNewVar_0 true)))))

(fn ConstructionScript)