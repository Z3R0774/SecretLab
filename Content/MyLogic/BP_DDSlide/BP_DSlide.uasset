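; BP_DSlide is a sliding door that moves a BPDoor component along its relative X axis when something overlaps its trigger volumes.
; Front and back triggers play separate timelines (Open and Timeline_1) and set Flag to record which was entered last.
; Leaving the door trigger reverses the timeline that Flag selects.
; Overlaps are not filtered by actor, and a third timeline, Timeline_0, is never triggered.
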(event OnComponentBeginOverlap(BP_FrontColision)
  (params (OverlappedComponent :type Primitive%20Component%20Object%20Reference) (OtherActor :type Actor%20Object%20Reference) (OtherComp :type Primitive%20Component%20Object%20Reference) (OtherBodyIndex :type Integer) (bFromSweep :type Boolean) (SweepResult :type Hit%20Result%20Structure%20%28by%20ref%29))
  (bind _bp_door (Variables|Default|GetBP_Door))
  (bind _relativelocation (Variables|/Script/Engine.SceneComponent|GetRelativeLocation _bp_door))
  (Variables|Default|SetFlag true)
  (bind _newtrack_0 (Timeline|Open Play)
    (:Update
      (Transformation|SetRelativeLocation _bp_door (Math|Vector|MakeVector _newtrack_0 (.y _relativelocation) (.z _relativelocation)) false false))))

(event OnComponentBeginOverlap(BP_BackColision)
  (params (OverlappedComponent :type Primitive%20Component%20Object%20Reference) (OtherActor :type Actor%20Object%20Reference) (OtherComp :type Primitive%20Component%20Object%20Reference) (OtherBodyIndex :type Integer) (bFromSweep :type Boolean) (SweepResult :type Hit%20Result%20Structure%20%28by%20ref%29))
  (bind _bp_door (Variables|Default|GetBP_Door))
  (bind _relativelocation (Variables|/Script/Engine.SceneComponent|GetRelativeLocation _bp_door))
  (Variables|Default|SetFlag false)
  (bind _newtrack_0 (Timeline|Timeline_1 Play)
    (:Update
      (Transformation|SetRelativeLocation _bp_door (Math|Vector|MakeVector _newtrack_0 (.y _relativelocation) (.z _relativelocation)) false false))))

(event OnComponentEndOverlap(BP_DoorColision)
  (params (OverlappedComponent :type Primitive%20Component%20Object%20Reference) (OtherActor :type Actor%20Object%20Reference) (OtherComp :type Primitive%20Component%20Object%20Reference) (OtherBodyIndex :type Integer))
  (bind _bp_door (Variables|Default|GetBP_Door))
  (bind _bp_door_2 (Variables|Default|GetBP_Door))
  (bind _relativelocation (Variables|/Script/Engine.SceneComponent|GetRelativeLocation _bp_door))
  (bind _relativelocation_2 (Variables|/Script/Engine.SceneComponent|GetRelativeLocation _bp_door_2))
  (if (Variables|Default|GetFlag)
    (bind _newtrack_0 (Timeline|Open Reverse)
      (:Update
        (Transformation|SetRelativeLocation _bp_door_2 (Math|Vector|MakeVector _newtrack_0 (.y _relativelocation_2) (.z _relativelocation_2)) false false)))
    (else
      (bind _newtrack_0_2 (Timeline|Timeline_1 Reverse)
        (:Update
          (Transformation|SetRelativeLocation _bp_door (Math|Vector|MakeVector _newtrack_0_2 (.y _relativelocation) (.z _relativelocation)) false false))))))

(fn ConstructionScript)